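; BP_Character is a simple player character with keyboard movement and mouse look.
; Tick polls W/S and A/D directly on player controller 0, avoiding input bindings for simplicity, which a comment flags as unsuitable for real projects.
; The keys add movement along the actor's forward and right vectors, with W and D taking priority over their opposites.
; Mouse axis events drive controller yaw and inverted-value pitch to rotate the character and camera.
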(event EventTick
  (params (DeltaSeconds :type Float%20%28single-precision%29))
  (bind _returnvalue (Game|GetPlayerController 0))
  (bind _returnvalue_2 (Game|GetPlayerController 0))
  ;[1 1 1] You shouldn't do this in actual projects, but we want make sure that we don't need any bindings for this simple character.
  (Utilities|FlowControl|Sequence
    (:then_0
      (if (Game|Player|IsInputKeyDown _returnvalue "W")
        (Pawn|Input|AddMovementInput (Transformation|GetActorForwardVector) 1.0 false)
        (elif (Game|Player|IsInputKeyDown _returnvalue "S")
          (Pawn|Input|AddMovementInput (Transformation|GetActorForwardVector) -1.0 false))))
    (:then_1
      (if (Game|Player|IsInputKeyDown _returnvalue_2 "D")
        (Pawn|Input|AddMovementInput (Transformation|GetActorRightVector) 1.0 false)
        (elif (Game|Player|IsInputKeyDown _returnvalue_2 "A")
          (Pawn|Input|AddMovementInput (Transformation|GetActorRightVector) -1.0 false))))))

(event Input|MouseEvents|MouseX
  (params (AxisValue :type Float%20%28single-precision%29))
  ;[1 1 1] Rotate character and camera.
  (Pawn|Input|AddControllerYawInput AxisValue))

(event Input|MouseEvents|MouseY
  (params (AxisValue :type Float%20%28single-precision%29))
  ;[1 1 1] Rotate character and camera.
  (Pawn|Input|AddControllerPitchInput (* AxisValue -1.0)))

(fn ConstructionScript)